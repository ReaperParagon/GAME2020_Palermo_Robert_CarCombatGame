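; Arena turret that fires Turret_Projectile_BP from its head toward TargetDirection on a looping ShootTime timer while its health is above zero.
; IncHealth applies health changes to a living turret and calls Death when health runs out.
; Death clears the head mesh, destroys the sphere component and decrements the turret count on the player's Vehicle_BP.
; Tick runs a visibility line trace from the head whose result is unused.
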(event EventBeginPlay
  (Utilities|Time|SetTimerbyFunctionName self "TurretShoot" (Variables|Default|GetShootTime) true))

(event EventTick
  (params (DeltaSeconds :type Float%20%28single-precision%29))
  (Collision|LineTraceByChannel (Transformation|GetWorldLocation (Variables|Default|GetMeshHead)) (* (Variables|Default|GetTargetDirection) 300) "TraceTypeQuery1" false 0 "None"))

(fn ConstructionScript)

(fn TurretShoot
  (bind _meshhead (Variables|Default|GetMeshHead))
  (bind _returnvalue (Transformation|GetWorldLocation _meshhead))
  (if (> (Variables|Default|GetTurretHealth) 0.0)
    (Game|SpawnActorfromClass "/Game/Maps/Arena_1/Blueprints/Turret_Projectile_BP.Turret_Projectile_BP_C" (Math|Transform|MakeTransform _returnvalue (Math|Rotator|FindLookatRotation _returnvalue (* (Variables|Default|GetTargetDirection) 100))) "AlwaysSpawn" 0 0)))

(fn IncHealth
  (params (inc :type Float%20%28single-precision%29))
  (if (> (Variables|Default|GetTurretHealth) 0.0)
    (Class|MyTurret|IncrementHealth inc)
    (if (<= (Variables|Default|GetTurretHealth) 0.0)
      (CallFunction|Death))))

(fn Death
  (Components|StaticMesh|SetStaticMesh (Variables|Default|GetMeshHead) 0)
  (Components|DestroyComponent (Variables|Default|GetSphere))
  (bind _asvehicle_bp (Utilities|Casting|CastToVehicle_BP (Game|Player|GetPlayerPawn 0)))
  (Class|MyWheeledVehicle|IncrementTurretCount _asvehicle_bp -1))