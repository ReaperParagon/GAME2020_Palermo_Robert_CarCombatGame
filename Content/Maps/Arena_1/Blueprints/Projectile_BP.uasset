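; Projectile actor that damages turrets on contact.
; Its Sphere overlap only responds when the other component is a sphere component on a MyTurret_BP, then lowers that turret's health by one, plays an attenuated hit sound at the Bullet's location and destroys itself.
; A timer started on BeginPlay calls LifeSpan by name to destroy the projectile after a fixed delay if nothing is hit.
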(event OnComponentBeginOverlap(Sphere)
  (params (OverlappedComponent :type Primitive%20Component%20Object%20Reference) (OtherActor :type Actor%20Object%20Reference) (OtherComp :type Primitive%20Component%20Object%20Reference) (OtherBodyIndex :type Integer) (bFromSweep :type Boolean) (SweepResult :type Hit%20Result%20Structure%20%28by%20ref%29))
  (Utilities|Casting|CastToSphereComponent OtherComp)
  (bind _asmy_turret_bp (Utilities|Casting|CastToMyTurret_BP OtherActor))
  (Default|IncHealth _asmy_turret_bp -1.0)
  (Audio|SpawnSoundatLocation "/Game/Sounds/Turret_Hit_Cue.Turret_Hit_Cue" (Transformation|GetWorldLocation (Variables|Default|GetBullet)) "0, 0, 0" 1.0 1.0 0.0 "/Game/Sounds/Hit_Attenuation.Hit_Attenuation" 0)
  (Actor|DestroyActor))

(event EventBeginPlay
  (Utilities|Time|SetTimerbyFunctionName self "LifeSpan" 8.0))

(fn ConstructionScript)

(fn LifeSpan
  (Actor|DestroyActor))